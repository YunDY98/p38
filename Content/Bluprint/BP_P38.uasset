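; BP_P38 is an airplane actor that spins its two propellers and drifts along the world X axis.
; Each Tick passes the Left and Right components to a shared RotatePropeller function, which rolls them locally at RSpeed.
; Tick then moves the whole actor by a constant world offset without sweeping.
; Both rotation and movement scale by delta seconds, keeping them frame-rate independent.
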(event EventBeginPlay)

(event Collision|EventActorBeginOverlap
  (params (OtherActor :type Actor%20Object%20Reference)))

(event EventTick
  (params (DeltaSeconds :type Float%20%28single-precision%29))
  ;[1 1 1] Left DO Rotation
  (CallFunction|RotatePropeller (Variables|Default|GetLeft))
  ;[1 1 1] Right DO Rotation
  (CallFunction|RotatePropeller (Variables|Default|GetRight))
  ;[1 1 1] Move To Airplane
  (Transformation|AddActorWorldOffset (Math|Vector|MakeVector (* (Utilities|Time|GetWorldDeltaSeconds) 1e+01) 0.0 0.0)))

(fn ConstructionScript)

(fn RotatePropeller
  (params (self2 :type Scene%20Component%20Object%20Reference))
  (Transformation|AddLocalRotation self2 (Math|Rotator|MakeRotator (* (Utilities|Time|GetWorldDeltaSeconds) (Variables|Default|GetRSpeed)) 0.0 0.0) false false))