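; BP_221024 is an actor that spins two propeller components, Left and Right, while drifting slowly along world X.
; Tick rolls both components locally by RSpeed scaled by frame time and offsets the actor at a fixed, frame-rate-independent speed.
; A RotatePropeller function holds the same rotation logic for any passed component, but Tick repeats it inline instead of calling it.
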(event EventBeginPlay)

(event Collision|EventActorBeginOverlap
  (params (OtherActor :type Actor%20Object%20Reference)))

(event EventTick
  (params (DeltaSeconds :type Float%20%28single-precision%29))
  (Transformation|AddLocalRotation (Variables|Default|GetLeft) (Math|Rotator|MakeRotator (* (Variables|Default|GetRSpeed) DeltaSeconds) 0.0 0.0) false false)
  (Transformation|AddLocalRotation (Variables|Default|GetRight) (Math|Rotator|MakeRotator (* (Variables|Default|GetRSpeed) (Utilities|Time|GetWorldDeltaSeconds)) 0.0 0.0) false false)
  (Transformation|AddActorWorldOffset (Math|Vector|MakeVector (* (Utilities|Time|GetWorldDeltaSeconds) 1e+01) 0.0 0.0)))

(fn ConstructionScript)

(fn RotatePropeller
  (params (self2 :type Scene%20Component%20Object%20Reference))
  (Transformation|AddLocalRotation self2 (Math|Rotator|MakeRotator (* (Utilities|Time|GetWorldDeltaSeconds) (Variables|Default|GetRSpeed)) 0.0 0.0) false false))